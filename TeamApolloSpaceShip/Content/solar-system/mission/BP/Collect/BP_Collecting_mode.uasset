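; BP_Collecting_mode runs a timed collecting mission, tracking a score and ending the round when time runs out.
; BeginPlay shows the WBP_PlayingCollect HUD and plays the MissionTime timeline in reverse as a countdown, converting its time to display text.
; AddToScore increments the score.
; When the timeline finishes, RaceCompletion pauses the game, replaces all widgets with the WBP_EndColl end screen and enables mouse-driven UI input.
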(event `self.ReceiveBeginPlay`
  (bind _returnvalue (`|CreateWidget` "/Game/solar-system/mission/UI/collect/WBP_PlayingCollect.WBP_PlayingCollect_C"))
  (`UserWidget.AddToViewport` _returnvalue 0)
  (bind (_direction _time) (`Timeline|Mission Time` :!via `ReverseFromEnd`)
    (:`Update`
      (set `self.MissionTime` (`KismetTextLibrary.Conv_StringToText` (`KismetStringLibrary.TimeSecondsToString` _time))))
    (:`Finished`
      (`self.RaceCompletion`))))

(fn `addToScore`
  (`/Engine/EditorBlueprintResources/StandardMacros.IncrementInt` (`self.Score`)))

(fn `RaceCompletion`
  (bind _returnvalue (`GameplayStatics.GetPlayerController` 0))
  (`GameplayStatics.SetGamePaused` true)
  (`WidgetLayoutLibrary.RemoveAllWidgets`)
  (bind _returnvalue_2 (`|CreateWidget` "/Game/solar-system/mission/UI/collect/WBP_EndColl.WBP_EndColl_C"))
  (`UserWidget.AddToViewport` _returnvalue_2 0)
  (set `PlayerController.bShowMouseCursor` true _returnvalue)
  (`WidgetBlueprintLibrary.SetInputMode_GameAndUIEx` _returnvalue _returnvalue_2 "DoNotLock" false))

(fn `UserConstructionScript`)