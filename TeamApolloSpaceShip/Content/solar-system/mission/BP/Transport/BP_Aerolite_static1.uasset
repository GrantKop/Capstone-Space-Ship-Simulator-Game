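; BP_Aerolite_static1 is an asteroid obstacle in the transport mission that damages the player's ship on contact.
; On BeginPlay it tags itself "Obstacle" and adds a RotatingMovement component with a random spin on each axis.
; The first overlap with ShipCharacter_User decrements ShipHealth on the game instance, with DoOnce blocking repeat hits.
; When health reaches zero, it calls RaceCompletion on the BP_TransporMode game mode.
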(event `self.ReceiveBeginPlay`
  (`KismetArrayLibrary.Array_Add` (`self.Tags`) "Obstacle")
  (bind _returnvalue (`AddComponent|NODE_AddRotatingMovementComponent-2`))
  (set `RotatingMovementComponent.RotationRate` (`KismetMathLibrary.MakeRotator` (`KismetMathLibrary.RandomFloatInRange` 0.0 25.0) (`KismetMathLibrary.RandomFloatInRange` 0.0 25.0) (`KismetMathLibrary.RandomFloatInRange` 0.0 25.0)) _returnvalue))

(event `self.ReceiveActorBeginOverlap`
  (params (OtherActor :type "Actor Object Reference"))
  (if (== (`GameplayStatics.GetObjectClass` OtherActor) "/Game/Ships/PlayerShip/ShipCharacter_User.ShipCharacter_User_C")
    (`/Engine/EditorBlueprintResources/StandardMacros.DoOnce` false
      (:`Completed`
        (bind _asmy_game_instance (cast `/Game/Blueprints/MyGameInstance` (`GameplayStatics.GetGameInstance`)))
        (bind _result (`/Engine/EditorBlueprintResources/StandardMacros.DecrementInt` (`/Game/Blueprints/MyGameInstance.shipHealth` _asmy_game_instance))
          (:`  `
            (if (<= _result 0)
              (bind _asbp_transpor_mode (cast `/Game/solar-system/mission/BP/Transport/BP_TransporMode` (`GameplayStatics.GetGameMode`)))
              (`/Game/solar-system/mission/BP/Transport/BP_TransporMode.RaceCompletion` _asbp_transpor_mode))))))))

(fn `UserConstructionScript`)