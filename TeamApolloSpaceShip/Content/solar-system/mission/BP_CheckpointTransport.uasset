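; Ring checkpoint for the transport and racing modes that counts down when the player's ship passes through it.
; A trigger overlap only counts if the ship's velocity does not point along the Arrow's forward vector, making the checkpoint directional.
; The current level name selects the game mode to notify: Racing uses BP_Racing_mode, other levels use BP_TransporMode.
; After notifying, it hides the ring and disables the trigger's overlap events.
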(event `self.ReceiveBeginPlay`)

(event `self.trigger.OnComponentBeginOverlap`
  (params (OverlappedComponent :type "PrimitiveComponent Object Reference") (OtherActor :type "Actor Object Reference") (OtherComp :type "PrimitiveComponent Object Reference") (OtherBodyIndex :type Integer) (bFromSweep :type Boolean) (SweepResult :type "HitResult Structure (by ref)"))
  (bind _returnvalue (`GameplayStatics.GetGameMode`))
  (bind _asship_character_user (cast `/Game/ShipCharacter_User` OtherActor))
  (if (<= (`KismetMathLibrary.Dot_VectorVector` (`self.GetVelocity` _asship_character_user) (`KismetMathLibrary.Conv_RotatorToVector` (`SceneComponent.K2_GetComponentRotation` (`self.Arrow`)))) 0.0)
    (bind _returnvalue_2 (`GameplayStatics.GetCurrentLevelName` true))
    (switch `name` (`KismetStringLibrary.Conv_StringToName` _returnvalue_2)
      (:`Default`
        (bind _asbp_transpor_mode (cast `/Game/solar-system/mission/BP/BP_TransporMode` _returnvalue))
        (`/Game/solar-system/mission/BP/BP_TransporMode.checkpointCountDown` _asbp_transpor_mode))
      (:`racing`
        (bind _asbp_racing_mode (cast `/Game/solar-system/mission/BP/BP_Racing_mode` _returnvalue))
        (`/Game/solar-system/mission/BP/BP_Racing_mode.checkpointCountDown` _asbp_racing_mode)))
    (`SceneComponent.SetHiddenInGame` (`self.ring`) true false)
    (set `PrimitiveComponent.bGenerateOverlapEvents` false (`self.trigger`))))

(fn `UserConstructionScript`)