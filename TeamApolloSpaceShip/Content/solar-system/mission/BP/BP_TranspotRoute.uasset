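; BP_TranspotRoute is a spline-based mission route actor for the solar-system game, shaped by placed checkpoints and able to scatter asteroids along itself.
; On BeginPlay it inserts each CheckpointArr actor's location as a world-space spline point, starting after the first point.
; SpawnStaticRock, not called within this Blueprint, spawns randomly offset, rotated and scaled BP_Aerolite_static rocks around every interior spline point, skipping spawns with unresolvable collisions.
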(event `self.ReceiveBeginPlay`
  (for (_array_element _array_index) (`self.CheckpointArr`)
    (`SplineComponent.AddSplinePointAtIndex` (`self.Spline`) (`self.K2_GetActorLocation` _array_element) (+ _array_index 1) "World" true)))

(fn `SpawnStaticRock`
  (bind _returnvalue (`KismetMathLibrary.RandomFloatInRange` 0.0 180.0))
  (bind _rocklocationoffset (`self.RockLocationOffset`))
  (bind _spline (`self.Spline`))
  (bind _returnvalue_2 (`KismetMathLibrary.RandomFloatInRange` (* _rocklocationoffset -1.0) _rocklocationoffset))
  (for _index (range 1 (+ (- (`SplineComponent.GetNumberOfSplinePoints` _spline) 2) 1))
    (for _ (range 1 (+ (`self.RockNumPerSPoint`) 1))
      (bind (_returnvalue_x _returnvalue_y _returnvalue_z) (`KismetMathLibrary.BreakVector` (`SplineComponent.GetLocationAtSplinePoint` _spline _index "World")))
      (`|SpawnActorFromClass` "/Game/solar-system/mission/BP_Aerolite_static.BP_Aerolite_static_C" (`KismetMathLibrary.MakeTransform` (`KismetMathLibrary.MakeVector` (+ _returnvalue_x _returnvalue_2) (+ _returnvalue_y _returnvalue_2) (+ _returnvalue_z _returnvalue_2)) (`KismetMathLibrary.MakeRotator` _returnvalue _returnvalue _returnvalue) (`KismetMathLibrary.Conv_DoubleToVector` (`KismetMathLibrary.RandomFloatInRange` 0.5 1.0))) "AdjustIfPossibleButDontSpawnIfColliding" "MultiplyWithRoot" null null))))

(fn `UserConstructionScript`)