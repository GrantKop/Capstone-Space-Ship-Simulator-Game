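; BP_CheckpointTransport is a one-shot ring checkpoint for the player ship in the transport mission mode.
; When a ShipCharacter_User overlaps the Trigger, it counts only if the ship's velocity has a zero or negative dot product with the Arrow's forward vector, enforcing pass direction.
; A valid pass calls CheckpointCountDown on BP_TransporMode, then hides the Ring and disables the Trigger's overlap events.
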(event `self.trigger.OnComponentBeginOverlap`
  (params (OverlappedComponent :type "PrimitiveComponent Object Reference") (OtherActor :type "Actor Object Reference") (OtherComp :type "PrimitiveComponent Object Reference") (OtherBodyIndex :type Integer) (bFromSweep :type Boolean) (SweepResult :type "HitResult Structure (by ref)"))
  (bind _asship_character_user (cast `/Game/Ships/PlayerShip/ShipCharacter_User` OtherActor))
  (if (<= (`KismetMathLibrary.Dot_VectorVector` (`self.GetVelocity` _asship_character_user) (`KismetMathLibrary.Conv_RotatorToVector` (`SceneComponent.K2_GetComponentRotation` (`self.Arrow`)))) 0.0)
    (bind _asbp_transpor_mode (cast `/Game/solar-system/mission/BP/Transport/BP_TransporMode` (`GameplayStatics.GetGameMode`)))
    (`/Game/solar-system/mission/BP/Transport/BP_TransporMode.checkpointCountDown` _asbp_transpor_mode)
    (`SceneComponent.SetHiddenInGame` (`self.ring`) true false)
    (set `PrimitiveComponent.bGenerateOverlapEvents` false (`self.trigger`))))

(fn `UserConstructionScript`)