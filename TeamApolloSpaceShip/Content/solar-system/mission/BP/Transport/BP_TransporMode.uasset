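; Game mode for the transport mission, a checkpoint race that ends when every checkpoint has been counted down.
; On BeginPlay it gathers all BP_CheckpointTransport actors, shows the playing widget and starts a Timeline that serves as the race clock text.
; CheckpointCountDown decrements the remaining count and at zero triggers RaceCompletion.
; RaceCompletion pauses the game, clears the SpawnRock timer, destroys an array of actors and swaps to the end screen with mouse input.
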(event `self.ReceiveBeginPlay`
  (bind _outactors (`GameplayStatics.GetAllActorsOfClass` "/Game/solar-system/mission/BP/Transport/BP_CheckpointTransport.BP_CheckpointTransport_C"))
  (bind _output_get (set `self.checkpointArr(gameMode)` _outactors))
  (bind _returnvalue (`KismetArrayLibrary.Array_Length` _output_get))
  (set `self.totalCheckpoints(gameMode)` _returnvalue)
  (set `self.checkpoint Left` _returnvalue)
  (bind _returnvalue_2 (`|CreateWidget` "/Game/solar-system/mission/UI/transportation/WBP_PlayingTransport.WBP_PlayingTransport_C"))
  (`UserWidget.AddToViewport` _returnvalue_2 0)
  (bind (_direction _time) (`Timeline|Timeline`)
    (:`Update`
      (set `self.RaceTime` (`KismetTextLibrary.Conv_StringToText` (`KismetStringLibrary.TimeSecondsToString` _time))))))

(fn `checkpointCountDown`
  (bind _result (`/Engine/EditorBlueprintResources/StandardMacros.DecrementInt` (`self.checkpoint Left`))
    (:`  `
      (if (== _result 0)
        (set `self.RaceComplete?` true)
        (`self.RaceCompletion`)))))

(fn `RaceCompletion`
  (bind _returnvalue (`GameplayStatics.GetPlayerController` 0))
  (`GameplayStatics.SetGamePaused` true)
  (`KismetSystemLibrary.K2_ClearTimer` null "SpawnRock")
  (for _array_element _
    (`/Engine/EditorBlueprintResources/StandardMacros.IsValid` _array_element
      (:`Is Valid`
        (`self.K2_DestroyActor` _array_element))))
  (`WidgetLayoutLibrary.RemoveAllWidgets`)
  (bind _returnvalue_2 (`|CreateWidget` "/Game/solar-system/mission/UI/transportation/WBP_End.WBP_End_C"))
  (`UserWidget.AddToViewport` _returnvalue_2 0)
  (set `PlayerController.bShowMouseCursor` true _returnvalue)
  (`WidgetBlueprintLibrary.SetInputMode_GameAndUIEx` _returnvalue _returnvalue_2 "DoNotLock" false))

(fn `UserConstructionScript`)