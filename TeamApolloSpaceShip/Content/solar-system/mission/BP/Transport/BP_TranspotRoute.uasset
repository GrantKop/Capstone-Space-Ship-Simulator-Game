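; Transport-route mission actor with logic to spawn floating asteroids (BP_Aerolite_float) around the player's ship.
; SpawnFloatingRock places a randomly scaled rock at a random offset from the ship mesh and stores it in RocksArr.
; Rock heading and InitSpeed derive from a reversed random offset vector, with Y adjusted by ship velocity to lead the target.
; The timed spawn loop is disconnected and BeginPlay only casts the GameInstance, so nothing here triggers spawning.
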(event `self.ReceiveBeginPlay`
  (cast `/Game/Blueprints/MyGameInstance` (`GameplayStatics.GetGameInstance`)))

(fn `SpawnFloatingRock`
  (bind _returnvalue (`KismetMathLibrary.RandomFloatInRange` -7500.0 7500.0))
  (bind _returnvalue_2 (`KismetMathLibrary.RandomFloatInRange` 2500.0 7500.0))
  (bind _returnvalue_3 (`KismetMathLibrary.RandomFloatInRange` 5000.0 15000.0))
  (bind (_returnvalue_x _returnvalue_y _returnvalue_z) (`KismetMathLibrary.BreakVector` (`KismetMathLibrary.MakeVector` _returnvalue_2 _returnvalue_3 _returnvalue)))
  (bind _returnvalue_4 (`GameplayStatics.GetActorOfClass` "/Game/Ships/PlayerShip/ShipCharacter_User.ShipCharacter_User_C"))
  (bind _scifi_fighter_ak5 (`/Game/Ships/PlayerShip/ShipCharacter_User.SciFi_Fighter_AK5` _returnvalue_4))
  (bind (_returnvalue_x_2 _returnvalue_y_2 _returnvalue_z_2) (`KismetMathLibrary.BreakVector` (`SceneComponent.K2_GetComponentLocation` _scifi_fighter_ak5)))
  (bind (_returnvalue_x_3 _returnvalue_y_3) (`KismetMathLibrary.BreakVector` (`SceneComponent.GetComponentVelocity` _scifi_fighter_ak5)))
  (bind _returnvalue_5 (* (`KismetMathLibrary.MakeVector` _returnvalue_x _returnvalue_y _returnvalue_z) (`KismetMathLibrary.MakeVector` -1.0 (* (/ (- _returnvalue_y (* 5.0 _returnvalue_y_3)) _returnvalue_y) -1.0) -1.0)))
  (bind _returnvalue_6 (`|SpawnActorFromClass` "/Game/solar-system/mission/BP_Aerolite_float.BP_Aerolite_float_C" (`KismetMathLibrary.MakeTransform` (`KismetMathLibrary.MakeVector` (+ _returnvalue_x_2 _returnvalue_2) (+ _returnvalue_y_2 _returnvalue_3) (+ _returnvalue_z_2 _returnvalue)) (`KismetMathLibrary.Conv_VectorToRotator` _returnvalue_5) (`KismetMathLibrary.Conv_DoubleToVector` (`KismetMathLibrary.RandomFloatInRange` 0.5 1.0))) "AdjustIfPossibleButAlwaysSpawn" "MultiplyWithRoot" null (/ (`KismetMathLibrary.VSize` _returnvalue_5) 3.0) null))
  (`KismetArrayLibrary.Array_Add` (`self.rocksArr`) _returnvalue_6))

(fn `UserConstructionScript`)