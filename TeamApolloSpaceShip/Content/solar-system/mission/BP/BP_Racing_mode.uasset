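; BP_Racing_mode runs a checkpoint race in the solar-system game, tracking race time and checkpoints left.
; BeginPlay gathers every BP_Checkpoint, numbers each one's NextIndex and, inside that same loop, creates the race HUD and plays the MissionTime timeline that formats RaceTime.
; CheckpointCountDown triggers RaceCompletion at zero, pausing the game and showing the end widget with mouse input.
; StopTImer halts the timeline if RaceComplete is set.
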(event `self.ReceiveBeginPlay`
  (bind _outactors (`GameplayStatics.GetAllActorsOfClass` "/Game/solar-system/mission/BP_Checkpoint.BP_Checkpoint_C"))
  (bind _output_get (set `self.checkpointArr(gameMode)` _outactors))
  (for (_array_element _array_index) _output_get
    (set `/Game/solar-system/mission/BP_Checkpoint.nextIndex` (+ _array_index 1) _array_element)
    (bind _output_get_2 (set `self.totalCheckpoints(gameMode)` (`KismetArrayLibrary.Array_Length` _output_get)))
    (set `self.checkpoint Left` _output_get_2)
    (bind _returnvalue (`|CreateWidget` "/Game/solar-system/mission/UI/WBP_PlayingRace.WBP_PlayingRace_C"))
    (`UserWidget.AddToViewport` _returnvalue 0)
    (bind (_direction _time) (`Timeline|Mission Time` :!label _label)
      (:`Update`
        (set `self.RaceTime` (`KismetTextLibrary.Conv_StringToText` (`KismetStringLibrary.TimeSecondsToString` _time)))))))

(event `StopTImer`
  (if (`self.RaceComplete?`)
    (goto _label :!via `Stop`)))

(fn `checkpointCountDown`
  (bind _result (`/Engine/EditorBlueprintResources/StandardMacros.DecrementInt` (`self.checkpoint Left`))
    (:`  `
      (if (== _result 0)
        (`self.RaceCompletion`)))))

(fn `RaceCompletion`
  (bind _returnvalue (`GameplayStatics.GetPlayerController` 0))
  (`GameplayStatics.SetGamePaused` true)
  (`WidgetLayoutLibrary.RemoveAllWidgets`)
  (bind _returnvalue_2 (`|CreateWidget` "/Game/solar-system/mission/UI/WBP_End.WBP_End_C"))
  (`UserWidget.AddToViewport` _returnvalue_2 0)
  (set `PlayerController.bShowMouseCursor` true _returnvalue)
  (`WidgetBlueprintLibrary.SetInputMode_GameAndUIEx` _returnvalue _returnvalue_2 "DoNotLock" false))

(fn `UserConstructionScript`)