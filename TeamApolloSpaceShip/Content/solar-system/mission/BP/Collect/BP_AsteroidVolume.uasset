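; Asteroid field volume for a collection mission, filling a box with random meshes and spawning the collectible object.
; The construction script adds about 500 individual static mesh components, using RandomTransform for location within the Volume extents, rotation and non-uniform scale.
; The layout is unseeded, so it changes whenever construction reruns.
; On BeginPlay it spawns BP_CollectionObj at a fixed Y offset from the PlayerStart, independent of the volume.
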(event `self.ReceiveBeginPlay`
  (bind _returnvalue (`GameplayStatics.GetActorOfClass` "/Script/Engine.PlayerStart"))
  (bind _returnvalue_2 (`self.GetTransform` _returnvalue))
  (`|SpawnActorFromClass` "/Game/solar-system/mission/BP/Collect/BP_CollectionObj.BP_CollectionObj_C" (`KismetMathLibrary.MakeTransform` (`KismetMathLibrary.MakeVector` (.x (.location _returnvalue_2)) (+ (.y (.location _returnvalue_2)) -800.0) (.z (.location _returnvalue_2))) (struct :`Yaw` 180.0)) "AdjustIfPossibleButAlwaysSpawn" "MultiplyWithRoot" null null))

(fn `RandomTransform`
  (returns (ReturnValue :type "Transform Structure"))
  (bind _returnvalue (`KismetMathLibrary.RandomFloatInRange` 0.1 5.0))
  (bind (_returnvalue_x _returnvalue_y _returnvalue_z) (`KismetMathLibrary.BreakVector` (`BoxComponent.GetScaledBoxExtent` (`self.Volume`))))
  (return (`KismetMathLibrary.MakeTransform` (+ (`KismetMathLibrary.MakeVector` (`KismetMathLibrary.RandomFloatInRange` (* _returnvalue_x -1.0) _returnvalue_x) (`KismetMathLibrary.RandomFloatInRange` (* _returnvalue_y -1.0) _returnvalue_y) (`KismetMathLibrary.RandomFloatInRange` (* _returnvalue_z -1.0) _returnvalue_z)) (`self.K2_GetActorLocation`)) (`KismetMathLibrary.RandomRotator` true) (`KismetMathLibrary.MakeVector` _returnvalue _returnvalue _returnvalue))))

(fn `UserConstructionScript`
  (for _ (range 501)
    (bind _returnvalue (`AddComponent|NODE_AddStaticMeshComponent-3`))
    (bind _returnvalue_2 (`self.RandomTransform`))
    (`SceneComponent.K2_SetWorldTransform` _returnvalue _returnvalue_2 false false)))