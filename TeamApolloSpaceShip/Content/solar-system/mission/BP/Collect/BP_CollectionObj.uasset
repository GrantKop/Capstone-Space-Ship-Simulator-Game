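; BP_CollectionObj is a collectible in the solar-system collecting mission that scores and respawns when its trigger is overlapped.
; Any overlap adds to the BP_Collecting_mode score, then moves the same actor to a random transform from BP_AsteroidVolume at fixed scale.
; Tick stores the yaw offset between player control rotation and direction to the object in TargetScreenLocation.
; A RandomLocation function builds transforms within Volume's extents, but the event graph never calls it.
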(event `self.ReceiveBeginPlay`)

(event `self.ReceiveTick`
  (params (DeltaSeconds :type "Float (single-precision)"))
  (bind _returnvalue (`GameplayStatics.GetPlayerCharacter` 0))
  (bind (_returnvalue_roll _returnvalue_pitch _returnvalue_yaw) (`KismetMathLibrary.BreakRotator` (`Pawn.GetControlRotation` _returnvalue)))
  (bind (_returnvalue_roll_2 _returnvalue_pitch_2 _returnvalue_yaw_2) (`KismetMathLibrary.BreakRotator` (`KismetMathLibrary.FindLookAtRotation` (`self.K2_GetActorLocation` _returnvalue) (`self.K2_GetActorLocation`))))
  (set `self.TargetScreenLocation` (- _returnvalue_yaw _returnvalue_yaw_2)))

(event `self.trigger.OnComponentBeginOverlap`
  (params (OverlappedComponent :type "PrimitiveComponent Object Reference") (OtherActor :type "Actor Object Reference") (OtherComp :type "PrimitiveComponent Object Reference") (OtherBodyIndex :type Integer) (bFromSweep :type Boolean) (SweepResult :type "HitResult Structure (by ref)"))
  (bind _asbp_collecting_mode (cast `/Game/solar-system/mission/BP/Collect/BP_Collecting_mode` (`GameplayStatics.GetGameMode`)))
  (`/Game/solar-system/mission/BP/Collect/BP_Collecting_mode.addToScore` _asbp_collecting_mode)
  (bind _returnvalue (`GameplayStatics.GetActorOfClass` "/Game/solar-system/mission/BP/Collect/BP_AsteroidVolume.BP_AsteroidVolume_C"))
  (bind _returnvalue_2 (`/Game/solar-system/mission/BP/Collect/BP_AsteroidVolume.RandomTransform` _returnvalue))
  (`self.K2_SetActorTransform` (`KismetMathLibrary.MakeTransform` (.location _returnvalue_2) (.rotation _returnvalue_2) (5.0 5.0 5.0)) true))

(fn `RandomLocation`
  (returns (ReturnValue :type "Transform Structure"))
  (bind (_returnvalue_x _returnvalue_y _returnvalue_z) (`KismetMathLibrary.BreakVector` (`BoxComponent.GetScaledBoxExtent` (`/Game/solar-system/mission/BP/Collect/BP_AsteroidVolume.Volume` (`self.volume`)))))
  (bind _returnvalue (* _returnvalue_z 0.75))
  (bind _returnvalue_2 (* _returnvalue_x 0.75))
  (bind _returnvalue_3 (* _returnvalue_y 0.75))
  (return (`KismetMathLibrary.MakeTransform` (+ (`KismetMathLibrary.MakeVector` (`KismetMathLibrary.RandomFloatInRange` (* _returnvalue_2 -1.0) _returnvalue_2) (`KismetMathLibrary.RandomFloatInRange` (* _returnvalue_3 -1.0) _returnvalue_3) (`KismetMathLibrary.RandomFloatInRange` (* _returnvalue -1.0) _returnvalue)) (`self.K2_GetActorLocation`)) (`KismetMathLibrary.RandomRotator` true) (2.0 2.0 2.0))))

(fn `UserConstructionScript`)