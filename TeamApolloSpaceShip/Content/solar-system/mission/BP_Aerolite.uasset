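; BP_Aerolite is an asteroid-like hazard in the solar-system mission that damages the player's ship on contact.
; Overlapping a ShipCharacter decrements ShipHealth in BP_GameInst and calls RaceCompletion on the BP_TansporMode game mode once health reaches zero or below.
; A MoveToShip event uses AI MoveTo to chase the ship, but the logic that finds the ship and calls it is disconnected and never runs.
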(event `self.ReceiveBeginPlay`)

(event `MoveToShip`
  (`|AIMoveTo` self (0.0 0.0 0.0) (`self.spaceShip`) 1.0
    (:`then`
      (`KismetSystemLibrary.PrintString` "success"))
    (:`OnFail`
      (`KismetSystemLibrary.PrintString` "failed"))))

(event `self.ReceiveActorBeginOverlap`
  (params (OtherActor :type "Actor Object Reference"))
  (cast `/Game/ShipCharacter` OtherActor)
  (bind _asbp_game_inst (cast `/Game/solar-system/BP_GameInst` (`GameplayStatics.GetGameInstance`)))
  (bind _result (`/Engine/EditorBlueprintResources/StandardMacros.DecrementInt` (`/Game/solar-system/BP_GameInst.shipHealth` _asbp_game_inst))
    (:`  `
      (if (<= _result 0)
        (bind _asbp_tanspor_mode (cast `/Game/solar-system/mission/BP/BP_TansporMode` (`GameplayStatics.GetGameMode`)))
        (`/Game/solar-system/mission/BP/BP_TansporMode.RaceCompletion` _asbp_tanspor_mode)))))

(fn `UserConstructionScript`)