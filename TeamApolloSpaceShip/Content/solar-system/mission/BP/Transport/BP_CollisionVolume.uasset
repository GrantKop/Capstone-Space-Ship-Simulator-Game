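; BP_CollisionVolume is a spawner actor that scatters static aerolite obstacles inside a box volume for the solar-system transport mission.
; On BeginPlay it loops over the Obstacles count, spawning BP_Aerolite_static1 at transforms from RandomTransform.
; That function picks a point within Volume1's scaled extents around the actor location, with random rotation and effectively fixed scale.
; Spawns adjust to avoid collisions or are skipped if still colliding.
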(event `self.ReceiveBeginPlay`
  (for _ (range (+ (`self.obstacles`) 1))
    (bind _returnvalue (`self.RandomTransform`))
    (`|SpawnActorFromClass` "/Game/solar-system/mission/BP/Transport/BP_Aerolite_static1.BP_Aerolite_static1_C" _returnvalue "AdjustIfPossibleButDontSpawnIfColliding" "MultiplyWithRoot" null null)))

(fn `RandomTransform`
  (returns (ReturnValue :type "Transform Structure"))
  (bind _returnvalue (`KismetMathLibrary.RandomFloatInRange` 1.5 1.5))
  (bind (_returnvalue_x _returnvalue_y _returnvalue_z) (`KismetMathLibrary.BreakVector` (`BoxComponent.GetScaledBoxExtent` (`self.Volume1`))))
  (return (`KismetMathLibrary.MakeTransform` (+ (`KismetMathLibrary.MakeVector` (`KismetMathLibrary.RandomFloatInRange` (* _returnvalue_x -1.0) _returnvalue_x) (`KismetMathLibrary.RandomFloatInRange` (* _returnvalue_y -1.0) _returnvalue_y) (`KismetMathLibrary.RandomFloatInRange` (* _returnvalue_z -1.0) _returnvalue_z)) (`self.K2_GetActorLocation`)) (`KismetMathLibrary.RandomRotator` true) (`KismetMathLibrary.MakeVector` _returnvalue _returnvalue _returnvalue))))

(fn `UserConstructionScript`)