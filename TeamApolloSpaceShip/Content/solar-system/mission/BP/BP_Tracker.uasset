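; BP_Tracker is an unfinished checkpoint tracker, apparently for a racing mission.
; BeginPlay caches BP_Racing_mode and runs ApplySettings, whose UpdateTimes function is an empty stub with unused medal-time variables.
; ActivateCheckpoint shows a checkpoint's ring and enables its trigger overlaps, but the start-sequence call and checkpoint-cleared bindings never run.
; CheckpointCheck compares the cleared checkpoint against TotalCheckpoints without acting on the result.
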(event `ApplySettings`
  ;[1 1 1] Start game settings
  (`self.Update Times` null))

(event `StartSequence`
  ;[1 1 1] Start Sequence
  (`self.Activate Checkpoint` null))

(event `CheckpointClear_Event`
  (params (NextCheckpoint :type Integer))
  ;[1 1 1] Start Sequence
  (`self.CheckpointCheck` NextCheckpoint)
  (if true
    _))

(event `self.ReceiveBeginPlay`
  ;[1 1 1] Get and promote to variable
  (bind _asbp_racing_mode (cast `/Game/solar-system/mission/BP/BP_Racing_mode` (`GameplayStatics.GetGameMode`)))
  (set `self.As BP Racing Mode` _asbp_racing_mode)
  (`self.ApplySettings`))

(fn `Activate Checkpoint`
  (params (`Next checkpoint` :type "/Game/solar-system/mission/BP_Checkpoint Object Reference"))
  (`SceneComponent.SetHiddenInGame` (`/Game/solar-system/mission/BP_Checkpoint.ring` `Next checkpoint`) false false)
  (set `PrimitiveComponent.bGenerateOverlapEvents` true (`/Game/solar-system/mission/BP_Checkpoint.trigger` `Next checkpoint`)))

(fn `CheckpointCheck`
  (params (`Local Checkpoint` :type Integer))
  (locals (L_Checkpoint :type Integer))
  (bind _output_get (set `local.L_Checkpoint` `Local Checkpoint`))
  (if (== _output_get (`self.Total Checkpoints`))
    _))

(fn `Update Times`
  (params (ring :type "StaticMeshComponent Object Reference")))

(fn `UserConstructionScript`)