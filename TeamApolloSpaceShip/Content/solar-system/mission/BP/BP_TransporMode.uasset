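; Game mode for the transport mission: counts BP_CheckpointTransport checkpoints, shows the HUD and sets asteroid hazards by difficulty.
; Easy spawns static route rocks, Norm loops delayed floating-rock spawns near the ship, aimed using its Y velocity, and Hard does both.
; CheckpointCountDown sets RaceComplete at zero, which lets StopTImer stop the race-time Timeline.
; RaceCompletion pauses, clears rocks and shows the end screen, but its call in CheckpointCountDown is disconnected.
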(event `self.ReceiveBeginPlay`
  (bind _outactors (`GameplayStatics.GetAllActorsOfClass` "/Game/solar-system/mission/BP_CheckpointTransport.BP_CheckpointTransport_C"))
  (bind _output_get (set `self.checkpointArr(gameMode)` _outactors))
  (bind _returnvalue (`KismetArrayLibrary.Array_Length` _output_get))
  (set `self.totalCheckpoints(gameMode)` _returnvalue)
  (set `self.checkpoint Left` _returnvalue)
  (bind _returnvalue_2 (`|CreateWidget` "/Game/solar-system/mission/UI/WBP_PlayingTransport.WBP_PlayingTransport_C"))
  (`UserWidget.AddToViewport` _returnvalue_2 0)
  (bind _asmy_game_instance (cast `/Game/Blueprints/MyGameInstance` (`GameplayStatics.GetGameInstance`)))
  (switch `string` (`/Game/Blueprints/MyGameInstance.CurrMissionDif` _asmy_game_instance)
    (:`Default`
      _)
    (:`easy`
      _)
    (:`norm`
      (`KismetSystemLibrary.Delay` (`self.RockSpawnTime`) :!label _label)
      (bind _returnvalue_3 (`GameplayStatics.GetActorOfClass` "/Game/Ships/PlayerShip/ShipCharacter_User.ShipCharacter_User_C"))
      (`self.SpawnFloatingRock` _returnvalue_3)
      (goto _label))
    (:`hard`
      (bind _returnvalue_4 (`GameplayStatics.GetActorOfClass` "/Game/solar-system/mission/BP/BP_TranspotRoute.BP_TranspotRoute_C"))
      (`/Game/solar-system/mission/BP/BP_TranspotRoute.SpawnStaticRock` _returnvalue_4)
      (`KismetSystemLibrary.Delay` (`self.RockSpawnTime`) :!label _label_2)
      (bind _returnvalue_5 (`GameplayStatics.GetActorOfClass` "/Game/Ships/PlayerShip/ShipCharacter_User.ShipCharacter_User_C"))
      (`self.SpawnFloatingRock` _returnvalue_5)
      (goto _label_2)))
  (bind _returnvalue_6 (`GameplayStatics.GetActorOfClass` "/Game/solar-system/mission/BP/BP_TranspotRoute.BP_TranspotRoute_C"))
  (`/Game/solar-system/mission/BP/BP_TranspotRoute.SpawnStaticRock` _returnvalue_6))

(event `StopTImer`
  (if (`self.RaceComplete?`)
    (bind (_direction _time) (`Timeline|Timeline` :!via `Stop`)
      (:`Update`
        (set `self.RaceTime` (`KismetTextLibrary.Conv_StringToText` (`KismetStringLibrary.TimeSecondsToString` _time)))))))

(fn `checkpointCountDown`
  (bind _result (`/Engine/EditorBlueprintResources/StandardMacros.DecrementInt` (`self.checkpoint Left`))
    (:`  `
      (if (== _result 0)
        (set `self.RaceComplete?` true)))))

(fn `RaceCompletion`
  (bind _returnvalue (`GameplayStatics.GetPlayerController` 0))
  (`GameplayStatics.SetGamePaused` true)
  (`KismetSystemLibrary.K2_ClearTimer` null "SpawnRock")
  (for _array_element (`self.rocksArr`)
    (`/Engine/EditorBlueprintResources/StandardMacros.IsValid` _array_element
      (:`Is Valid`
        (`self.K2_DestroyActor` _array_element))))
  (`WidgetLayoutLibrary.RemoveAllWidgets`)
  (bind _returnvalue_2 (`|CreateWidget` "/Game/solar-system/mission/UI/WBP_End.WBP_End_C"))
  (`UserWidget.AddToViewport` _returnvalue_2 0)
  (set `PlayerController.bShowMouseCursor` true _returnvalue)
  (`WidgetBlueprintLibrary.SetInputMode_GameAndUIEx` _returnvalue _returnvalue_2 "DoNotLock" false))

(fn `SpawnFloatingRock`
  (params (shipChar :type "/Game/Ships/PlayerShip/ShipCharacter_User Object Reference"))
  (bind _returnvalue (`KismetMathLibrary.RandomFloatInRange` -7500.0 7500.0))
  (bind _returnvalue_2 (`KismetMathLibrary.RandomFloatInRange` 2500.0 7500.0))
  (bind _returnvalue_3 (`KismetMathLibrary.RandomFloatInRange` 5000.0 15000.0))
  (bind _scifi_fighter_ak5 (`/Game/Ships/PlayerShip/ShipCharacter_User.SciFi_Fighter_AK5` shipChar))
  (bind (_returnvalue_x _returnvalue_y _returnvalue_z) (`KismetMathLibrary.BreakVector` (`KismetMathLibrary.MakeVector` _returnvalue_2 _returnvalue_3 _returnvalue)))
  (bind (_returnvalue_x_2 _returnvalue_y_2 _returnvalue_z_2) (`KismetMathLibrary.BreakVector` (`SceneComponent.K2_GetComponentLocation` _scifi_fighter_ak5)))
  (bind (_returnvalue_x_3 _returnvalue_y_3) (`KismetMathLibrary.BreakVector` (`SceneComponent.GetComponentVelocity` _scifi_fighter_ak5)))
  (bind _returnvalue_4 (* (`KismetMathLibrary.MakeVector` _returnvalue_x _returnvalue_y _returnvalue_z) (`KismetMathLibrary.MakeVector` -1.0 (* (/ (- _returnvalue_y (* 5.0 _returnvalue_y_3)) _returnvalue_y) -1.0) -1.0)))
  (bind _returnvalue_5 (`|SpawnActorFromClass` "/Game/solar-system/mission/BP_Aerolite_float.BP_Aerolite_float_C" (`KismetMathLibrary.MakeTransform` (`KismetMathLibrary.MakeVector` (+ _returnvalue_x_2 _returnvalue_2) (+ _returnvalue_y_2 _returnvalue_3) (+ _returnvalue_z_2 _returnvalue)) (`KismetMathLibrary.Conv_VectorToRotator` _returnvalue_4) (`KismetMathLibrary.Conv_DoubleToVector` (`KismetMathLibrary.RandomFloatInRange` 0.5 1.0))) "AdjustIfPossibleButAlwaysSpawn" "MultiplyWithRoot" null (/ (`KismetMathLibrary.VSize` _returnvalue_4) 3.0) null))
  (`KismetArrayLibrary.Array_Add` (`self.rocksArr`) _returnvalue_5))

(fn `UserConstructionScript`)