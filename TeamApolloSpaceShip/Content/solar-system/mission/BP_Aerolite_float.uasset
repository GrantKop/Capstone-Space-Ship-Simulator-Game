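; BP_Aerolite_float is a floating meteor hazard that damages the player's ship in the solar-system mission.
; The construction script sets projectile speed from InitSpeed, and BeginPlay adds a random spin before destroying the actor after a fixed delay.
; Its first overlap with ShipCharacter_User decrements ShipHealth in the game instance, calling the game mode's RaceCompletion when health is depleted.
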(event `self.ReceiveBeginPlay`
  (bind _returnvalue (`AddComponent|NODE_AddRotatingMovementComponent-2`))
  (set `RotatingMovementComponent.RotationRate` (`KismetMathLibrary.MakeRotator` (`KismetMathLibrary.RandomFloatInRange` 0.0 180.0) (`KismetMathLibrary.RandomFloatInRange` 0.0 180.0) (`KismetMathLibrary.RandomFloatInRange` 0.0 180.0)) _returnvalue)
  (`KismetSystemLibrary.Delay` 8.0)
  (`self.K2_DestroyActor`))

(event `self.ReceiveActorBeginOverlap`
  (params (OtherActor :type "Actor Object Reference"))
  (if (== (`GameplayStatics.GetObjectClass` OtherActor) "/Game/ShipCharacter_User.ShipCharacter_User_C")
    (`/Engine/EditorBlueprintResources/StandardMacros.DoOnce` false
      (:`Completed`
        (bind _asbp_game_inst (cast `/Game/solar-system/BP_GameInst` (`GameplayStatics.GetGameInstance`)))
        (bind _result (`/Engine/EditorBlueprintResources/StandardMacros.DecrementInt` (`/Game/solar-system/BP_GameInst.shipHealth` _asbp_game_inst))
          (:`  `
            (if (<= _result 0)
              (bind _asbp_transpor_mode (cast `/Game/solar-system/mission/BP/BP_TransporMode` (`GameplayStatics.GetGameMode`)))
              (`/Game/solar-system/mission/BP/BP_TransporMode.RaceCompletion` _asbp_transpor_mode))))))))

(fn `UserConstructionScript`
  (bind _projectilemovement (`self.ProjectileMovement`))
  (bind _initspeed (`self.initSpeed`))
  (set `ProjectileMovementComponent.InitialSpeed` _initspeed _projectilemovement)
  (set `ProjectileMovementComponent.MaxSpeed` _initspeed _projectilemovement))